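; BP_Target_+Speed is a shootable target actor that grants the player a speed boost.
; When a FirstPersonProjectile begins overlapping its TargetCollision, it calls SpeedBoost on player 0's FirstPersonCharacter and plays a 2D sound cue.
; The target does not destroy or disable itself, and the boost logic itself lives in the character.
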(event `self.TargetCollision.OnComponentBeginOverlap`
  (params (OverlappedComponent :type "PrimitiveComponent Object Reference") (OtherActor :type "Actor Object Reference") (OtherComp :type "PrimitiveComponent Object Reference") (OtherBodyIndex :type Integer) (bFromSweep :type Boolean) (SweepResult :type "HitResult Structure (by ref)"))
  ;[1 1 1] Boost Speed if Shot By Projectile
  (cast `/Game/FirstPersonBP/Blueprints/FirstPersonProjectile` OtherActor)
  (bind _asfirst_person_character (cast `/Game/FirstPersonBP/Blueprints/FirstPersonCharacter` (`GameplayStatics.GetPlayerCharacter` 0)))
  (`/Game/FirstPersonBP/Blueprints/FirstPersonCharacter.SpeedBoost` _asfirst_person_character)
  (`GameplayStatics.PlaySound2D` "/Engine/VREditor/Sounds/VR_open_Cue.VR_open_Cue" 2.0 1.0 0.0 null null))

(fn `UserConstructionScript`
  (`parent.UserConstructionScript`))