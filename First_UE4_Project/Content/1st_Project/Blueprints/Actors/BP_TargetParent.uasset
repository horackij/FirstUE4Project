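; BP_TargetParent is a base shootable target that pops in with a sound and scale animation, then shrinks and destroys itself after its LifeTime.
; Stand-alone targets start hidden without collision and spawn once when the FirstPersonCharacter enters their TriggerVolume; others spawn on BeginPlay.
; An overlapping FirstPersonProjectile is destroyed, triggering an explosion effect and sound before the target destroys itself.
; No score is awarded here, despite the PtValue display component.
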(event `self.ReceiveBeginPlay`
  (if (`self.IsStandAloneTarget?`)
    ;[1 1 1] Stand Alone Target - Hide Target and Remove Collision
    (`SceneComponent.SetVisibility` (`self.PtValue`) false false)
    (`SceneComponent.SetVisibility` (`self.Target`) false false)
    (`SceneComponent.SetVisibility` (`self.SpotLight`) false false)
    (`PrimitiveComponent.SetCollisionEnabled` (`self.TargetCollision`) "NoCollision")
    (else
      ;[1 1 1] Target Spawn
      (`|ExecutionSequence` :!label _label
        (:`then_0`
          (`GameplayStatics.PlaySound2D` "/Engine/EditorSounds/GamePreview/PossessPlayer_Cue.PossessPlayer_Cue" 1.0 1.0 0.0 null null)
          (bind (_direction _scale) (`Timeline|SpawnAnimation` :!label _label_2)
            (:`Update`
              (`/Engine/EditorBlueprintResources/StandardMacros.IsValid` self
                (:`Is Valid`
                  (`SceneComponent.SetRelativeScale3D` (`self.TargetCollision`) (`KismetMathLibrary.Conv_DoubleToVector` _scale)))))))
        (:`then_1`
          (`KismetSystemLibrary.Delay` (`self.LifeTime`))
          (`|ExecutionSequence`
            (:`then_0`
              (goto _label_2 :!via `Reverse`))
            (:`then_1`
              (`KismetSystemLibrary.Delay` 0.3)
              (`self.K2_DestroyActor`))))))))

(event `self.TriggerVolume.OnComponentBeginOverlap`
  (params (OverlappedComponent :type "PrimitiveComponent Object Reference") (OtherActor :type "Actor Object Reference") (OtherComp :type "PrimitiveComponent Object Reference") (OtherBodyIndex :type Integer) (bFromSweep :type Boolean) (SweepResult :type "HitResult Structure (by ref)"))
  ;[1 1 1] Spawn as Stand Alone Target
  (cast `/Game/FirstPersonBP/Blueprints/FirstPersonCharacter` OtherActor)
  (if (`self.IsStandAloneTarget?`)
    (`/Engine/EditorBlueprintResources/StandardMacros.DoOnce` false
      (:`Completed`
        (`SceneComponent.SetVisibility` (`self.SpotLight`) true false)
        (`SceneComponent.SetVisibility` (`self.Target`) true false)
        (`SceneComponent.SetVisibility` (`self.PtValue`) true false)
        (`PrimitiveComponent.SetCollisionEnabled` (`self.TargetCollision`) "QueryOnly")
        (goto _label)))))

(event `self.TargetCollision.OnComponentBeginOverlap`
  (params (OverlappedComponent :type "PrimitiveComponent Object Reference") (OtherActor :type "Actor Object Reference") (OtherComp :type "PrimitiveComponent Object Reference") (OtherBodyIndex :type Integer) (bFromSweep :type Boolean) (SweepResult :type "HitResult Structure (by ref)"))
  (bind _returnvalue (`SceneComponent.K2_GetComponentLocation` (`self.TargetCollision`)))
  ;[1 1 1] Destroy Projectile and Target When Hit
  (bind _asfirst_person_projectile (cast `/Game/FirstPersonBP/Blueprints/FirstPersonProjectile` OtherActor))
  (`self.K2_DestroyActor` _asfirst_person_projectile)
  (`GameplayStatics.SpawnEmitterAtLocation` "/Game/StarterContent/Particles/P_Explosion.P_Explosion" _returnvalue (struct) (1.5 1.5 1.5))
  (`GameplayStatics.PlaySoundAtLocation` "/Game/StarterContent/Audio/Explosion_Cue.Explosion_Cue" _returnvalue (struct) 1.0 1.0 0.0 null null null)
  (`KismetSystemLibrary.Delay` 0.05)
  (`self.K2_DestroyActor`))

(fn `UserConstructionScript`)