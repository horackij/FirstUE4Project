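; BP_Target_+Time is a shootable target that extends the game clock when the player hits it with a projectile.
; The TargetCollision begin-overlap event filters for FirstPersonProjectile, then adds BonusTime to GameTimeLimit on BP_GameMode_GamePlay and plays a 2D confirmation sound.
; The graph itself neither destroys the target nor guards against repeat hits.
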(event `self.TargetCollision.OnComponentBeginOverlap`
  (params (OverlappedComponent :type "PrimitiveComponent Object Reference") (OtherActor :type "Actor Object Reference") (OtherComp :type "PrimitiveComponent Object Reference") (OtherBodyIndex :type Integer) (bFromSweep :type Boolean) (SweepResult :type "HitResult Structure (by ref)"))
  ;[1 1 1] Add Time if Player Destroys with Projectile
  (cast `/Game/FirstPersonBP/Blueprints/FirstPersonProjectile` OtherActor)
  (bind _asbp_game_mode_game_play (cast `/Game/1st_Project/Blueprints/Framework/BP_GameMode_GamePlay` (`GameplayStatics.GetGameMode`)))
  (set `/Game/1st_Project/Blueprints/Framework/BP_GameMode_GamePlay.GameTimeLimit` (+ (`/Game/1st_Project/Blueprints/Framework/BP_GameMode_GamePlay.GameTimeLimit` _asbp_game_mode_game_play) (`self.BonusTime`)) _asbp_game_mode_game_play)
  (`GameplayStatics.PlaySound2D` "/Engine/VREditor/Sounds/VR_confirm_Cue.VR_confirm_Cue" 1.0 1.0 0.0 null null))

(fn `UserConstructionScript`
  (`parent.UserConstructionScript`))