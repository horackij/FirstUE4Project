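; Player controller Blueprint that toggles the pause menu and game pause when P is pressed.
; An IsGamePaused flag picks the branch: pausing creates a new WBP_PauseMenu, shows the cursor and pauses, while unpausing removes the widget and reverses this.
; Pausing uses Game and UI input mode focused on the menu, intended to keep the key recognized while paused.
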(event `Key|P` :paused true
  (params (Key :type "Key Structure"))
  ;[1 1 1] Pause/Unpause Functionality
  (:`Pressed`
    (if (`self.IsGamePaused`)
      (set `self.IsGamePaused` false)
      (`Widget.RemoveFromParent` (stale _returnvalue))
      (set `self.bShowMouseCursor` false)
      (`WidgetBlueprintLibrary.SetInputMode_GameOnly` self)
      (`GameplayStatics.SetGamePaused` false)
      (else
        (set `self.IsGamePaused` true)
        (bind _returnvalue (`|CreateWidget` "/Game/1st_Project/UI/WBP_PauseMenu.WBP_PauseMenu_C"))
        (`UserWidget.AddToViewport` _returnvalue 0)
        (set `self.bShowMouseCursor` true)
        (`WidgetBlueprintLibrary.SetInputMode_GameAndUIEx` self _returnvalue) ; Must Set This so we can be recognized again when the game is paused
        (`GameplayStatics.SetGamePaused` true)))))

(fn `UserConstructionScript`)